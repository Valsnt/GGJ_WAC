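; Duck shooting-gallery target with front, middle and back ducks that start moving when a ThirdPersonCharacter enters its trigger box.
; Each duck has its own timeline driving relative side-to-side and up-down position, ping-ponging endlessly through a direction flag checked on finish.
; A Projectile overlapping a duck's collision sets that duck's hit flag and swaps its material to the hit version, without stopping its movement.
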(event `self.Box.OnComponentBeginOverlap`
  (params (OverlappedComponent :type "PrimitiveComponent Object Reference") (OtherActor :type "Actor Object Reference") (OtherComp :type "PrimitiveComponent Object Reference") (OtherBodyIndex :type Integer) (bFromSweep :type Boolean) (SweepResult :type "HitResult Structure (by ref)"))
  (cast `/Game/ThirdPersonBP/Blueprints/ThirdPersonCharacter` OtherActor)
  (`self.StartDuckies`))

(event `FD_Start`
  (set `self.ForwardF` true)
  (bind (_direction _l_r _u_d) (`Timeline|Timeline_0` :!via `PlayFromStart` :!label _label)
    (:`Update`
      (`SceneComponent.K2_SetRelativeLocation` (`self.FDuck`) (`KismetMathLibrary.MakeVector` 0.0 _l_r _u_d) false false))
    (:`Finished`
      (if (`self.ForwardF`)
        (`self.FD_Reverse`)
        (else
          (`self.FD_Start`))))))

(event `FD_Reverse`
  (set `self.ForwardF` false)
  (goto _label :!via `Reverse`))

(event `MD_Star`
  (set `self.ForwardM` true)
  (bind (_direction _l_r _u_d) (`Timeline|Timeline_1` :!via `PlayFromStart` :!label _label_2)
    (:`Update`
      (`SceneComponent.K2_SetRelativeLocation` (`self.MDuck`) (`KismetMathLibrary.MakeVector` 100.0 _l_r _u_d) false false))
    (:`Finished`
      (if (`self.ForwardM`)
        (`self.MD_Reverse`)
        (else
          (`self.MD_Star`))))))

(event `MD_Reverse`
  (set `self.ForwardM` false)
  (goto _label_2 :!via `ReverseFromEnd`))

(event `BD_Start`
  (set `self.ForwardB` true)
  (bind (_direction _l_r _u_d) (`Timeline|Timeline_2` :!via `PlayFromStart` :!label _label_3)
    (:`Update`
      (`SceneComponent.K2_SetRelativeLocation` (`self.BDuck`) (`KismetMathLibrary.MakeVector` -110.0 _l_r _u_d) false false))
    (:`Finished`
      (if (`self.ForwardB`)
        (`self.BD_Reverse`)
        (else
          (`self.BD_Start`))))))

(event `BD_Reverse`
  (set `self.ForwardB` false)
  (goto _label_3 :!via `ReverseFromEnd`))

(event `self.FDuckCol.OnComponentBeginOverlap`
  (params (OverlappedComponent :type "PrimitiveComponent Object Reference") (OtherActor :type "Actor Object Reference") (OtherComp :type "PrimitiveComponent Object Reference") (OtherBodyIndex :type Integer) (bFromSweep :type Boolean) (SweepResult :type "HitResult Structure (by ref)"))
  (cast `/Game/ThirdPersonBP/Blueprints/Projectile` OtherActor)
  (set `self.DuckFHit` true)
  (`PrimitiveComponent.SetMaterial` (`self.FDuck`) 0 "/Game/Meshes/Duck/DUCK_2transp_HIt.DUCK_2transp_HIt"))

(event `self.MDuckCol.OnComponentBeginOverlap`
  (params (OverlappedComponent :type "PrimitiveComponent Object Reference") (OtherActor :type "Actor Object Reference") (OtherComp :type "PrimitiveComponent Object Reference") (OtherBodyIndex :type Integer) (bFromSweep :type Boolean) (SweepResult :type "HitResult Structure (by ref)"))
  (cast `/Game/ThirdPersonBP/Blueprints/Projectile` OtherActor)
  (set `self.DuckMHit` true)
  (`PrimitiveComponent.SetMaterial` (`self.MDuck`) 0 "/Game/Meshes/Duck/DUCK_2transp_HIt.DUCK_2transp_HIt"))

(event `self.BDuckCol.OnComponentBeginOverlap`
  (params (OverlappedComponent :type "PrimitiveComponent Object Reference") (OtherActor :type "Actor Object Reference") (OtherComp :type "PrimitiveComponent Object Reference") (OtherBodyIndex :type Integer) (bFromSweep :type Boolean) (SweepResult :type "HitResult Structure (by ref)"))
  (cast `/Game/ThirdPersonBP/Blueprints/Projectile` OtherActor)
  (set `self.DuckBHit` true)
  (`PrimitiveComponent.SetMaterial` (`self.BDuck`) 0 "/Game/Meshes/Duck/DUCK_2transp_HIt.DUCK_2transp_HIt"))

(fn `StartDuckies`
  (`self.BD_Start`)
  (`self.FD_Start`)
  (`self.MD_Star`))

(fn `UserConstructionScript`)